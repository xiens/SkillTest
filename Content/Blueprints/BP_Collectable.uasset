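; BP_Collectable is a pickup actor that so far only prints a debug message when the player overlaps its sphere.
; The overlap passes through an IsPlayerOverlap check set to use once.
; The construction script caches the mesh's relative location and centers the sphere on it.
; A timeline meant to bob and spin the mesh is present but never triggered, so the collectable does not animate.
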(event OnComponentBeginOverlap(Sphere)
  (params (OverlappedComponent :type Primitive%20Component%20Object%20Reference) (OtherActor :type Actor%20Object%20Reference) (OtherComp :type Primitive%20Component%20Object%20Reference) (OtherBodyIndex :type Integer) (bFromSweep :type Boolean) (SweepResult :type Hit%20Result%20Structure%20%28by%20ref%29))
  (Utilities|IsPlayerOverlap OtherActor true
    (:true
      (Development|PrintString "Overlaped Player"))))

(event EventBeginPlay)

(event Collision|EventActorBeginOverlap
  (params (OtherActor :type Actor%20Object%20Reference)))

(event EventTick
  (params (DeltaSeconds :type Float%20%28single-precision%29)))

(fn ConstructionScript
  (bind _output_get (Variables|Default|SetStertLoc (Variables|/Script/Engine.SceneComponent|GetRelativeLocation (Variables|Default|GetStaticMesh))))
  (Transformation|SetRelativeLocation (Variables|Default|GetSphere) _output_get false false))